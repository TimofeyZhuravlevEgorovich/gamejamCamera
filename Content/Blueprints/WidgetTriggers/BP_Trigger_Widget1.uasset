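; BP_Trigger_Widget1 is an overlap trigger that briefly shows the BPW_Hint1 hint widget on screen.
; On ActorBeginOverlap it checks that ActorOverlapped is valid, then creates the widget for player controller 0 and adds it to the viewport.
; After a three-second delay it removes the widget; nothing in the graph stops later overlaps from showing the hint again.
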(event EventBeginPlay
  (|CallParentFunction) ; This node is disabled and will not be called.\nDrag off pins to build functionality.
)

(event Collision|EventActorBeginOverlap
  (params (OtherActor :type Actor%20Object%20Reference))
  (|CallParentFunction OtherActor)
  (Variables|Default|GetActorOverlapped
    (:then
      (bind _returnvalue (UserInterface|CreateWidget "/Game/Blueprints/HUD/BPW_Hint1.BPW_Hint1_C" (Game|GetPlayerController 0)))
      (Variables|Default|SetWidget1 _returnvalue)
      (UserInterface|Viewport|AddtoViewport (Variables|Default|GetWidget1) 0)
      (Utilities|FlowControl|Delay 3.0)
      (Widget|RemovefromParent (Variables|Default|GetWidget1)))
    (:else)))

(fn ConstructionScript
  (|CallParentFunction))