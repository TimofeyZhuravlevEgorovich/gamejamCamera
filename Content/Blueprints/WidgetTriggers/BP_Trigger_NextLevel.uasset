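; Trigger actor that moves the game on to the final cutscene level when overlapped.
; On overlap it runs the parent handler, then continues only if the ActorOverlapped variable is valid.
; It puts a BPW_BlackScreen widget on the viewport, waits a short random delay, then opens LevelFinalCutscene by a hardcoded name.
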(event EventBeginPlay
  (|CallParentFunction) ; This node is disabled and will not be called.\nDrag off pins to build functionality.
)

(event Collision|EventActorBeginOverlap
  (params (OtherActor :type Actor%20Object%20Reference))
  (|CallParentFunction OtherActor)
  (Variables|Default|GetActorOverlapped
    (:then
      (bind _returnvalue (UserInterface|CreateWidget "/Game/Blueprints/HUD/BPW_BlackScreen.BPW_BlackScreen_C" (Game|GetPlayerController 0)))
      (Variables|Default|SetNewVar _returnvalue)
      (UserInterface|Viewport|AddtoViewport (Variables|Default|GetNewVar) 0)
      (Utilities|FlowControl|Delay (Math|Random|RandomFloatinRange 1.5 4.0))
      (Game|OpenLevel(byName) "LevelFinalCutscene"))
    (:else)))

(event EventTick
  (params (DeltaSeconds :type Float%20%28single-precision%29))
  (|CallParentFunction DeltaSeconds) ; This node is disabled and will not be called.\nDrag off pins to build functionality.
)

(fn ConstructionScript
  (|CallParentFunction))