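; BP_CameraBase is an interactable trigger actor that shows a text prompt while a BP_CharacterBase overlaps it.
; Overlap events store the character and toggle readiness and prompt visibility.
; Each tick, the text rotates toward that character's camera.
; Interact prints a debug message and sets IsAdd when ready, blocking later overlap activation, but returns true in both branches.
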(event EventBeginPlay
  (Rendering|SetVisibility (Variables|Default|GetTextRender) false false))

(event Collision|EventActorBeginOverlap
  (params (OtherActor :type Actor%20Object%20Reference))
  (if (not (Variables|Default|GetIsAdd))
    (bind _asbp_character_base (Utilities|Casting|CastToBP_CharacterBase OtherActor))
    (Variables|Default|SetCharacterInBox _asbp_character_base)
    (Rendering|SetVisibility (Variables|Default|GetTextRender) true false)
    (Variables|Default|SetIsReadyToInteract true)
    (Variables|Default|SetIsLookAtPlayerCamera true)))

(event EventTick
  (params (DeltaSeconds :type Float%20%28single-precision%29))
  (CallFunction|LookatPlayerCamera))

(event Collision|EventActorEndOverlap
  (params (OtherActor :type Actor%20Object%20Reference))
  (Utilities|Casting|CastToBP_CharacterBase OtherActor)
  (Variables|Default|SetCharacterInBox 0)
  (Rendering|SetVisibility (Variables|Default|GetTextRender) false false)
  (Variables|Default|SetIsReadyToInteract false)
  (Variables|Default|SetIsLookAtPlayerCamera false))

(fn ConstructionScript)

(fn LookatPlayerCamera
  (if (Variables|Default|GetIsLookatPlayerCamera)
    (bind _characterinbox (Variables|Default|GetCharacterInBox)
      (:then
        (Variables|Default|SetL_CameraLocation (Transformation|GetWorldLocation (Variables|/Game/Blueprints/Character/BP_CharacterBase.BP_CharacterBase_C|GetCamera _characterinbox)))
        (Transformation|SetWorldRotation (Variables|Default|GetTextRender) (Math|Rotator|FindLookatRotation (Transformation|GetWorldLocation (Variables|Default|GetTextRender)) (Variables|Default|GetL_CameraLocation)) false false))
      (:else))))

(fn Interact
  (if (Variables|Default|GetIsReadyToInteract)
    (Development|PrintString "success")
    (Variables|Default|SetIsAdd true)
    (return true)
    (else
      (return true))))