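; BP_CharacterBase is a character Blueprint that adds head bob through camera shakes.
; Every Tick, HeadBob checks velocity and CanJump, then starts a shake on player controller 0.
; The Walk shake plays when moving below a speed threshold while able to jump.
; All other cases, including faster movement, start the Idle shake.
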(event Custom|HeadBob
  (bind _returnvalue (Transformation|GetVelocity))
  (bind _returnvalue_2 (Math|Vector|VectorLength _returnvalue))
  (if (and (> _returnvalue_2 0.0) (Character|CanJump))
    (if (< _returnvalue_2 3e+02)
      (Game|Feedback|ClientStartCameraShake (Game|GetPlayerController 0) "/Game/Blueprints/Character/Headbob/walk.walk_C" 1.0 "CameraLocal" "0, 0, 0")
      (else
        (Game|Feedback|ClientStartCameraShake (Game|GetPlayerController 0) "/Game/Blueprints/Character/Headbob/idle.idle_C" 1.0 "CameraLocal" "0, 0, 0")))
    (else
      (Game|Feedback|ClientStartCameraShake (Game|GetPlayerController 0) "/Game/Blueprints/Character/Headbob/idle.idle_C" 1.0 "CameraLocal" "0, 0, 0"))))

(event EventTick
  (params (DeltaSeconds :type Float%20%28single-precision%29))
  (CallFunction|HeadBob))

(fn ConstructionScript)