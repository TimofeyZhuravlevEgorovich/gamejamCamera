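; BP_PlayerController is a player controller that turns axis input into look and movement for the controlled pawn.
; UD and LR axes feed pitch and yaw input at half strength.
; Forward/Backward and Left/Right add movement along forward and right vectors built from control rotation yaw only, so camera pitch does not affect direction.
; The Left/Right axis value is negated before it is applied.
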(event Input|AxisEvents|InputAxisLeft/Right
  (params (AxisValue :type Float%20%28single-precision%29))
  (Pawn|Input|AddMovementInput (Pawn|GetControlledPawn) (Math|Vector|GetRightVector (Math|Rotator|MakeRotator 0.0 0.0 (.Yaw (Math|Rotator|BreakRotator (Pawn|GetControlRotation :!class /Script/Engine.Controller))))) (* AxisValue -1.0) false))

(event Input|AxisEvents|InputAxisForward/Backward
  (params (AxisValue :type Float%20%28single-precision%29))
  (Pawn|Input|AddMovementInput (Pawn|GetControlledPawn) (Math|Vector|GetForwardVector (Math|Rotator|MakeRotator 0.0 0.0 (.Yaw (Math|Rotator|BreakRotator (Pawn|GetControlRotation :!class /Script/Engine.Controller))))) AxisValue false))

(event Input|AxisEvents|InputAxisLR
  (params (AxisValue :type Float%20%28single-precision%29))
  (Pawn|Input|AddControllerYawInput (Pawn|GetControlledPawn) (/ AxisValue 2.0)))

(event Input|AxisEvents|InputAxisUD
  (params (AxisValue :type Float%20%28single-precision%29))
  (Pawn|Input|AddControllerPitchInput (Pawn|GetControlledPawn) (/ AxisValue 2.0)))

(fn ConstructionScript)