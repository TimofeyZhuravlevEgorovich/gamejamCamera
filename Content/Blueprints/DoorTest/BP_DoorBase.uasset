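; BP_DoorBase is a hinged door that a BP_CharacterBase can open and close while inside its overlap area.
; Overlap enables interaction and shows a text render that turns to face that character's camera every tick.
; Interact toggles a timeline that swings the door's yaw up to a maximum angle, guarded against mid-swing input, with a creak sound on opening only.
; The construction script presets the rotation from IsDoorOpen.
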(event Custom|OpenDoor
  (if (not (Variables|Default|GetInProgress))
    (if (not (Variables|Default|GetIsDoorOpen))
      (Audio|PlaySoundatLocation "/Game/Sounds/CUE/MetalDoorCreak_Cue.MetalDoorCreak_Cue" (Transformation|GetActorLocation) "0, 0, 0" 1.0 1.0 0.0 0 0 0 0)
      (bind (_direction _dooropen) (Timeline|Timeline Play)
        (:Update
          (Variables|Default|SetInProgress true)
          (Transformation|SetRelativeRotation (Variables|Default|GetScene) (Math|Rotator|MakeRotator 0.0 0.0 (* _dooropen (Variables|Default|GetMaxDoorAngleOpen))) false false))
        (:Finished
          (Variables|Default|SetInProgress false)
          (switch Utilities|FlowControl|Switch|SwitchonETimelineDirection _direction
            (:Forward
              (Variables|Default|SetIsDoorOpen true))
            (:Backward
              (Variables|Default|SetIsDoorOpen false))))))))

(event Custom|CloseDoor
  (if (not (Variables|Default|GetInProgress))
    (if (Variables|Default|GetIsDoorOpen)
      (bind (_direction _dooropen) (Timeline|Timeline ReverseFromEnd)
        (:Update
          (Variables|Default|SetInProgress true)
          (Transformation|SetRelativeRotation (Variables|Default|GetScene) (Math|Rotator|MakeRotator 0.0 0.0 (* _dooropen (Variables|Default|GetMaxDoorAngleOpen))) false false))
        (:Finished
          (Variables|Default|SetInProgress false)
          (switch Utilities|FlowControl|Switch|SwitchonETimelineDirection _direction
            (:Forward
              (Variables|Default|SetIsDoorOpen true))
            (:Backward
              (Variables|Default|SetIsDoorOpen false))))))))

(event EventBeginPlay
  (Rendering|SetVisibility (Variables|Default|GetTextRender) false false))

(event EventTick
  (params (DeltaSeconds :type Float%20%28single-precision%29))
  (CallFunction|LookatPlayerCamera))

(event Collision|EventActorBeginOverlap
  (params (OtherActor :type Actor%20Object%20Reference))
  (bind _asbp_character_base (Utilities|Casting|CastToBP_CharacterBase OtherActor))
  (Variables|Default|SetCharacterInBox _asbp_character_base)
  (Rendering|SetVisibility (Variables|Default|GetTextRender) true false)
  (Variables|Default|SetIsReadyToInteract true)
  (Variables|Default|SetIsLookAtPlayerCamera true))

(event Collision|EventActorEndOverlap
  (params (OtherActor :type Actor%20Object%20Reference))
  (Utilities|Casting|CastToBP_CharacterBase OtherActor)
  (Variables|Default|SetCharacterInBox 0)
  (Rendering|SetVisibility (Variables|Default|GetTextRender) false false)
  (Variables|Default|SetIsReadyToInteract false)
  (Variables|Default|SetIsLookAtPlayerCamera false))

(fn ConstructionScript
  (Transformation|SetRelativeRotation (Variables|Default|GetScene) (Math|Rotator|MakeRotator 0.0 0.0 (Math|Float|SelectFloat (Variables|Default|GetMaxDoorAngleOpen) 0.0 (Variables|Default|GetIsDoorOpen))) false false))

(fn LookatPlayerCamera
  (if (Variables|Default|GetIsLookatPlayerCamera)
    (bind _characterinbox (Variables|Default|GetCharacterInBox)
      (:then
        (LocalVariables|SetL_CameraLocation (Transformation|GetWorldLocation (Variables|/Game/Blueprints/Character/BP_CharacterBase.BP_CharacterBase_C|GetCamera _characterinbox)))
        (Transformation|SetWorldRotation (Variables|Default|GetTextRender) (Math|Rotator|FindLookatRotation (Transformation|GetWorldLocation (Variables|Default|GetTextRender)) (LocalVariables|GetL_CameraLocation)) false false))
      (:else))))

(fn Interact
  (if (Variables|Default|GetIsReadyToInteract)
    (if (Variables|Default|GetIsDoorOpen)
      (CallFunction|CloseDoor)
      (return true)
      (else
        (CallFunction|OpenDoor)
        (return true)))
    (else
      (return false))))