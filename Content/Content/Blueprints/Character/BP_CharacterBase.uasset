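; Base player character with a tablet item, interaction and camera-shake head bob.
; When the backpack holds the tablet quest item, its mesh shows and an input toggles a timeline equip that opens a 3D widget UI with mouse cursor.
; A second timeline swaps the tablet screen for a camera widget, gated by per-camera access.
; An overlap sphere caches the BPI_Interact actor that ActionUse triggers.
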(event OnComponentBeginOverlap(InteractSphere)
  (params (OverlappedComponent :type Primitive%20Component%20Object%20Reference) (OtherActor :type Actor%20Object%20Reference) (OtherComp :type Primitive%20Component%20Object%20Reference) (OtherBodyIndex :type Integer) (bFromSweep :type Boolean) (SweepResult :type Hit%20Result%20Structure%20%28by%20ref%29))
  (if (Utilities|DoesObjectImplementInterface OtherActor "/Game/Blueprints/Interface/BPI_Interact.BPI_Interact_C")
    (Variables|Default|SetActorToInteract OtherActor)))

(event OnComponentEndOverlap(InteractSphere)
  (params (OverlappedComponent :type Primitive%20Component%20Object%20Reference) (OtherActor :type Actor%20Object%20Reference) (OtherComp :type Primitive%20Component%20Object%20Reference) (OtherBodyIndex :type Integer))
  (Variables|Default|SetActorToInteract 0))

(event Custom|HeadBob
  (bind _returnvalue (Transformation|GetVelocity))
  (bind _returnvalue_2 (Math|Vector|VectorLength _returnvalue))
  (if (> _returnvalue_2 0.0)
    (if (< _returnvalue_2 3e+02)
      (Game|Feedback|ClientStartCameraShake (Game|GetPlayerController 0) "/Game/Blueprints/Character/Headbob/walk.walk_C" 1.0 "CameraLocal" "0, 0, 0")
      (else
        (Game|Feedback|ClientStartCameraShake (Game|GetPlayerController 0) "/Game/Blueprints/Character/Headbob/idle.idle_C" 1.0 "CameraLocal" "0, 0, 0")))
    (else
      (Game|Feedback|ClientStartCameraShake (Game|GetPlayerController 0) "/Game/Blueprints/Character/Headbob/idle.idle_C" 1.0 "CameraLocal" "0, 0, 0"))))

(event Custom|CheckTabletEquip
  (bind _cube (Variables|Default|GetCube))
  (if (not (Utilities|Set|Contains (Variables|/Game/Blueprints/Components/BP_BackpackComponent.BP_BackpackComponent_C|GetQuestItem (Variables|Default|GetBP_BackpackComponent)) (Variables|Default|GetTabletName)))
    (Rendering|SetVisibility _cube false false)
    (else
      (Rendering|SetVisibility _cube true false))))

(event Custom|TestTabletClose
  (bind _returnvalue (Game|GetPlayerController 0))
  (bind _returnvalue_2 (Game|GetPlayerController 0))
  (if (Variables|Default|GetTabletTaken)
    (Rendering|SetVisibility (Variables|Default|GetWidget) false false)
    (Input|SetInputModeGameOnly _returnvalue false)
    (Variables|/Script/Engine.PlayerController|SetbShowMouseCursor _returnvalue false)
    (if (not (Variables|Default|GetInProgress))
      (bind (_direction _tabletequip) (Timeline|TabletEquip ReverseFromEnd)
        (:Update
          (Variables|Default|SetInProgress true)
          (Transformation|SetRelativeLocation (Variables|Default|GetCube) _tabletequip false false))
        (:Finished
          (Variables|Default|SetInProgress false)
          (switch Utilities|FlowControl|Switch|SwitchonETimelineDirection _direction
            (:Forward
              (Variables|Default|SetTabletTaken true)
              (Rendering|SetVisibility (Variables|Default|GetWidget) true false)
              (Input|SetInputModeUIOnly _returnvalue_2 (Variables|Default|GetWidgetREF) "LockInFullscreen" false)
              (Variables|/Script/Engine.PlayerController|SetbShowMouseCursor _returnvalue_2 true))
            (:Backward
              (Variables|Default|SetTabletTaken false))))))))

(event Custom|Open_Camera
  (params (Number :type Integer))
  (if (Utilities|Array|Get(acopy) (Variables|Default|GetCameraAccess) Number)
    (if (not (Variables|Default|GetInProgressUI))
      (bind (_direction _changeswidgets) (Timeline|TestTimeline PlayFromStart)
        (:Update
          (Variables|Default|SetInProgressUI true)
          (Transformation|SetRelativeLocation (Variables|Default|GetWidget) _changeswidgets false false))
        (:Finished
          (Variables|Default|SetInProgressUI false)
          (switch Utilities|FlowControl|Switch|SwitchonETimelineDirection _direction
            (:Forward
              (Rendering|SetVisibility (Variables|Default|GetWidget1) true false)
              (Rendering|SetVisibility (Variables|Default|GetWidget) false false))
            (:Backward
              (Rendering|SetVisibility (Variables|Default|GetWidget1) false false)
              (Rendering|SetVisibility (Variables|Default|GetWidget) true false))))))))

(event Custom|Close_Camera
  (bind (_direction _changeswidgets) (Timeline|TestTimeline ReverseFromEnd)
    (:Update
      (Variables|Default|SetInProgressUI true)
      (Transformation|SetRelativeLocation (Variables|Default|GetWidget) _changeswidgets false false))
    (:Finished
      (Variables|Default|SetInProgressUI false)
      (switch Utilities|FlowControl|Switch|SwitchonETimelineDirection _direction
        (:Forward
          (Rendering|SetVisibility (Variables|Default|GetWidget1) true false)
          (Rendering|SetVisibility (Variables|Default|GetWidget) false false))
        (:Backward
          (Rendering|SetVisibility (Variables|Default|GetWidget1) false false)
          (Rendering|SetVisibility (Variables|Default|GetWidget) true false))))))

(event EventBeginPlay
  (bind _widget (Variables|Default|GetWidget))
  (Utilities|FlowControl|Sequence
    (:then_0
      (Rendering|SetVisibility _widget false false))
    (:then_1
      (bind _returnvalue (Game|ConstructObjectfromClass _widget "/Game/Camera/Tablet_WBP.Tablet_WBP_C"))
      (bind _output_get (Variables|Default|SetWidgetREF _returnvalue))
      (UserInterface|SetWidget _widget _output_get))
    (:then_2
      (bind _returnvalue_2 (Game|ConstructObjectfromClass (Variables|Default|GetWidget1) "/Game/Camera/Tablet_cam_WBP.Tablet_cam_WBP_C"))
      (bind _output_get_2 (Variables|Default|SetWidgetCam _returnvalue_2))
      (UserInterface|SetWidget (Variables|Default|GetWidget1) _output_get_2))))

(event EventTick
  (params (DeltaSeconds :type Float%20%28single-precision%29))
  (CallFunction|HeadBob)
  (CallFunction|CheckTabletEquip))

(event Input|ActionEvents|InputActionTakeTablet
  (params (Key :type Key%20Structure :default "None"))
  (bind _returnvalue (Game|GetPlayerController 0))
  (bind _returnvalue_2 (Game|GetPlayerController 0))
  (:Pressed
    (if (Utilities|Set|Contains (Variables|/Game/Blueprints/Components/BP_BackpackComponent.BP_BackpackComponent_C|GetQuestItem (Variables|Default|GetBP_BackpackComponent)) (Variables|Default|GetTabletName))
      (if (not (Variables|Default|GetTabletTaken))
        (if (not (Variables|Default|GetInProgress))
          (bind (_direction _tabletequip) (Timeline|TabletEquip PlayFromStart)
            (:Update
              (Variables|Default|SetInProgress true)
              (Transformation|SetRelativeLocation (Variables|Default|GetCube) _tabletequip false false))
            (:Finished
              (Variables|Default|SetInProgress false)
              (switch Utilities|FlowControl|Switch|SwitchonETimelineDirection _direction
                (:Forward
                  (Variables|Default|SetTabletTaken true)
                  (Rendering|SetVisibility (Variables|Default|GetWidget) true false)
                  (Input|SetInputModeUIOnly _returnvalue_2 (Variables|Default|GetWidgetREF) "LockInFullscreen" false)
                  (Variables|/Script/Engine.PlayerController|SetbShowMouseCursor _returnvalue_2 true))
                (:Backward
                  (Variables|Default|SetTabletTaken false))))))
        (else
          (Rendering|SetVisibility (Variables|Default|GetWidget) false false)
          (Input|SetInputModeGameOnly _returnvalue false)
          (Variables|/Script/Engine.PlayerController|SetbShowMouseCursor _returnvalue false)
          (if (not (Variables|Default|GetInProgress))
            (Timeline|TabletEquip ReverseFromEnd)))))))

(fn ConstructionScript)

(fn ActionUse
  (bind _actortointeract (Variables|Default|GetActorToInteract)
    (:then
      (Class|BPIInteract|Interact(Message) _actortointeract))
    (:else)))